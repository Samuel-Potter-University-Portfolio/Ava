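; BP_Monster is an AI monster character that roars and holds still when it sees the player.
; On BeginPlay it caches the skeletal mesh's anim instance as BP_MonsterAnim.
; OnSeePlayer passes the roar duration to the animator's Roar, then disables the CharacterMovement component's tick for that same duration to freeze movement before re-enabling it.
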(event `self.ReceiveBeginPlay`
  (bind _asbp_monster_anim (cast `/Game/Characters/Monster/BP_MonsterAnim` (`SkeletalMeshComponent.GetAnimInstance` (`self.SkeletalMesh`))))
  (set `self.Animator` _asbp_monster_anim))

(event `self.OnSeePlayer`
  (params (player :type "AvaCharacter Object Reference"))
  (`/Game/Characters/Monster/BP_MonsterAnim.Roar` (`self.Animator`) (`self.Raw Time`))
  ;[1 0.3614 0.3216] Prevent movement for duration of raw
  (`ActorComponent.SetComponentTickEnabled` (`self.CharacterMovement`) false)
  (`KismetSystemLibrary.Delay` (`self.Raw Time`))
  (`ActorComponent.SetComponentTickEnabled` (`self.CharacterMovement`) true))

(fn `UserConstructionScript`)